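; Door Blueprint that records its closed position at BeginPlay and derives an open position 200 units above it.
; Activate and Deactivate set the current location as the start, pick the open or closed position as the end, and raise CanMove.
; No movement logic appears in these graphs, which only set that state.
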(event `self.ReceiveBeginPlay`
  (bind (_returnvalue_x _returnvalue_y _returnvalue_z) (`KismetMathLibrary.BreakVector` (`self.K2_GetActorLocation`)))
  (set `self.closePos` (`self.K2_GetActorLocation`))
  (set `self.openPos` (`KismetMathLibrary.MakeVector` _returnvalue_x _returnvalue_y (+ _returnvalue_z 200.0))))

(fn `Activate`
  (set `self.startPosition` (`self.K2_GetActorLocation`))
  (set `self.endPosition` (`self.openPos`))
  (set `self.canMove` true))

(fn `Deactivate`
  (set `self.startPosition` (`self.K2_GetActorLocation`))
  (set `self.endPosition` (`self.closePos`))
  (set `self.canMove` true))

(fn `UserConstructionScript`
  (`parent.UserConstructionScript`))
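; Moving platform Blueprint that cycles through a looping list of Positions, starting at the first one.
; On BeginPlay, it splits TimeToGoAll evenly across the position count unless UseTimeToGo is set.
; Each Tick calls the parent, then, whenever CanMove is false, advances wrapped indices to set the next start and end positions and re-enables CanMove.
; The interpolation itself is not in this graph.
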(event `self.ReceiveBeginPlay`
  (`self.K2_SetActorLocation` (`|GetArrayItem` (`self.positions`)))
  (if (not (`self.useTimeToGo`))
    (set `self.timeToGo` (/ (`self.timeToGoAll`) (`KismetArrayLibrary.Array_Length` (`self.positions`))))))

(event `self.ReceiveTick`
  (params (DeltaSeconds :type "Float (single-precision)"))
  (`parent.ReceiveTick` DeltaSeconds)
  (if (not (`self.canMove`))
    (`/Engine/EditorBlueprintResources/StandardMacros.IncrementInt` (`self.nextPosIndex`)
      (:`  `
        (`/Engine/EditorBlueprintResources/StandardMacros.IncrementInt` (`self.currentIndex`)
          (:`  `
            (set `self.startPosition` (`|GetArrayItem` (`self.positions`) (mod (`self.currentIndex`) (`KismetArrayLibrary.Array_Length` (`self.positions`)))))
            (set `self.endPosition` (`|GetArrayItem` (`self.positions`) (mod (`self.nextPosIndex`) (`KismetArrayLibrary.Array_Length` (`self.positions`)))))
            (set `self.canMove` true)))))))

(fn `UserConstructionScript`
  (`parent.UserConstructionScript`))
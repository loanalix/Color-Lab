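; Moving platform Blueprint that travels through an array of positions, either looping continuously or step by step in response to state changes.
; Continuous mode runs while activated; step mode moves forward on activation and back on deactivation by swapping current and next indices.
; Tick picks each segment's endpoints with modulo wrapping, then delegates to the parent Tick while CanMove is set.
; Segment time can be an even share of a total duration.
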(event `self.ReceiveBeginPlay`
  (`self.K2_SetActorLocation` (`|GetArrayItem` (`self.positions`)))
  (if (not (`self.useTimeToGo`))
    (set `self.timeToGo` (/ (`self.timeToGoAll`) (`KismetArrayLibrary.Array_Length` (`self.positions`))))))

(event `self.ReceiveTick`
  (params (DeltaSeconds :type "Float (single-precision)"))
  (if (`self.IsActive`)
    (if (`self.canMove`)
      (`parent.ReceiveTick` DeltaSeconds)
      (elif (`self.goStepByStep`)
        (if (`self.goToPrev`)
          (set `self.goToPrev` false)
          (`self.swapInts` (`self.nextPosIndex`) (`self.currentIndex`))
          (set `self.startPosition` (`self.K2_GetActorLocation`) :!label _label)
          (set `self.endPosition` (`|GetArrayItem` (`self.positions`) (mod (`self.nextPosIndex`) (`KismetArrayLibrary.Array_Length` (`self.positions`)))))
          (set `self.canMove` true)
          (if (`self.goToPrev`)
            (`self.swapInts` (`self.nextPosIndex`) (`self.currentIndex`)))
          (elif (`self.goToNext`)
            (set `self.goToNext` false)
            (`/Engine/EditorBlueprintResources/StandardMacros.IncrementInt` (`self.nextPosIndex`) :!label _label_2
              (:`  `
                (`/Engine/EditorBlueprintResources/StandardMacros.IncrementInt` (`self.currentIndex`)
                  (:`  `
                    (goto _label)))))))
        (else
          (goto _label_2))))))

(event `/Game/Blueprints/BPI_Activable.OnStateChanged`
  (params (IsActivated :type Boolean) (emitter :type "Actor Object Reference"))
  (if IsActivated
    (set `self.IsActive` true)
    (if (`self.goStepByStep`)
      (set `self.goToNext` true)
      (set `self.canMove` false)
      (set `self.timeAtStart` 0.0))
    (elif (`self.goStepByStep`)
      (set `self.IsActive` true)
      (set `self.goToPrev` true)
      (set `self.canMove` false)
      (set `self.timeAtStart` 0.0)
      (else
        (set `self.IsActive` false)))))

(fn `swapInts`
  (params (first :type Integer) (second :type Integer))
  (set `self.tempSwap` first)
  (set `self.nextPosIndex` second)
  (set `self.currentIndex` (`self.tempSwap`)))

(fn `UserConstructionScript`
  (`parent.UserConstructionScript`))
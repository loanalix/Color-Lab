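; Actor that moves in a straight line from a start position to an end position over a set duration.
; While CanMove is true, Tick records the start time, then calls Move each frame to lerp the location by elapsed time without sweeping.
; Once the duration has passed, it clears CanMove and the start time, without snapping to the exact end position.
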(event `self.ReceiveTick`
  (params (DeltaSeconds :type "Float (single-precision)"))
  (if (`self.canMove`)
    (if (== (`self.timeAtStart`) 0.0)
      (set `self.timeAtStart` (`GameplayStatics.GetTimeSeconds`))
      (elif (<= (/ (- (`GameplayStatics.GetTimeSeconds`) (`self.timeAtStart`)) (`self.timeToGo`)) 1.0)
        (`self.Move`)
        (else
          (set `self.canMove` false)
          (set `self.timeAtStart` 0.0))))))

(fn `Move`
  (`self.K2_SetActorLocation` (`KismetMathLibrary.VLerp` (`self.startPosition`) (`self.endPosition`) (/ (- (`GameplayStatics.GetTimeSeconds`) (`self.timeAtStart`)) (`self.timeToGo`)))))

(fn `UserConstructionScript`)
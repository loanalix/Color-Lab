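; Trigger zone that moves the game to another room when a Pawn enters and sends any other actor to a target location.
; For a Pawn, the box overlap deactivates a linked object, calls ChangeLevel on bp_MyGameState with the target room ID, then disables the zone's collision.
; For other actors, it makes the first-person player release its held object and teleports the overlapping actor to TargetActor's location.
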(event `self.Box.OnComponentBeginOverlap`
  (params (OverlappedComponent :type "PrimitiveComponent Object Reference") (OtherActor :type "Actor Object Reference") (OtherComp :type "PrimitiveComponent Object Reference") (OtherBodyIndex :type Integer) (bFromSweep :type Boolean) (SweepResult :type "HitResult Structure (by ref)"))
  ;[1 1 1] Change level
  (cast `Pawn` OtherActor
    (:`then`
      (message `/Game/Blueprints/BPI_Activable.OnStateChanged` (`self.ObjectToActivate`) false null)
      (bind _asbp_my_game_state (cast `/Game/Blueprints/UI/bp_MyGameState` (`GameplayStatics.GetGameState`)))
      (`/Game/Blueprints/UI/bp_MyGameState.ChangeLevel` _asbp_my_game_state (`self.TargetRoomID`))
      (`self.SetActorEnableCollision` false))
    (:`CastFailed`
      (bind _asbp_first_person_character (cast `/Game/FirstPerson/Blueprints/BP_FirstPersonCharacter` (`GameplayStatics.GetPlayerCharacter` 0)))
      (`/Game/FirstPerson/Blueprints/BP_FirstPersonCharacter.Release Object` _asbp_first_person_character)
      (`self.K2_SetActorLocation` OtherActor (`self.K2_GetActorLocation` (`self.TargetActor`)) false false))))

(fn `UserConstructionScript`)
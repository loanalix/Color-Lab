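; bp_ColorLight is a light Blueprint whose Cube mesh switches between blue, green, purple and red materials.
; ChangeColor compares the linear form of the given color against Blue, Green, Purple and Red in a nested branch chain, then sets the matching material on slot 0.
; Any other color leaves the material unchanged, and the construction script is empty.
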(fn `ChangeColor`
  (params (Color :type "Color Structure"))
  (if (== (`KismetMathLibrary.Conv_ColorToLinearColor` Color) (`KismetMathLibrary.Conv_ColorToLinearColor` (`self.Blue`)))
    (`PrimitiveComponent.SetMaterial` (`self.Cube`) 0 "/Game/Materials/M_LightBlue.M_LightBlue")
    (elif (== (`KismetMathLibrary.Conv_ColorToLinearColor` Color) (`KismetMathLibrary.Conv_ColorToLinearColor` (`self.Green`)))
      (`PrimitiveComponent.SetMaterial` (`self.Cube`) 0 "/Game/Materials/M_LightGreen.M_LightGreen")
      (elif (== (`KismetMathLibrary.Conv_ColorToLinearColor` Color) (`KismetMathLibrary.Conv_ColorToLinearColor` (`self.Purple`)))
        (`PrimitiveComponent.SetMaterial` (`self.Cube`) 0 "/Game/Materials/M_LightPurple.M_LightPurple")
        (elif (== (`KismetMathLibrary.Conv_ColorToLinearColor` Color) (`KismetMathLibrary.Conv_ColorToLinearColor` (`self.Red`)))
          (`PrimitiveComponent.SetMaterial` (`self.Cube`) 0 "/Game/Materials/M_LightRed.M_LightRed"))))))

(fn `UserConstructionScript`)
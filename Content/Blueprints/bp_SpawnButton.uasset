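; bp_SpawnButton is an interactable button that relays presses to the objects in its SignalReceivers list.
; InteractOnce plays the push animation, then sends OnReceiveSignalMessage to each receiver that implements the bpi_signalReeiver interface.
; InteractConstant sends OnReceiveConstantSignalMessage the same way, without the animation.
; Both messages pass the button and its Id, and any spawning is left to the receivers.
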(event `self.InteractOnce`
  (`ActorSequenceComponent.PlaySequence` (`self.pushAnimation`))
  (for _array_element (`self.signalReceivers`)
    (bind _asbpi_signal_reeiver (cast `/Game/Blueprints/bpi_signalReeiver` _array_element))
    (message `/Game/Blueprints/bpi_signalReeiver.OnReceiveSignal` (`KismetSystemLibrary.Conv_InterfaceToObject` _asbpi_signal_reeiver) self (`self.id`))))

(event `self.InteractConstant`
  (for _array_element (`self.signalReceivers`)
    (bind _asbpi_signal_reeiver (cast `/Game/Blueprints/bpi_signalReeiver` _array_element))
    (message `/Game/Blueprints/bpi_signalReeiver.OnReceiveConstantSignal` (`KismetSystemLibrary.Conv_InterfaceToObject` _asbpi_signal_reeiver) self (`self.id`))))

(fn `UserConstructionScript`)
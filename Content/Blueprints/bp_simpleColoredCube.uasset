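; A physics cube actor that changes color by cycling through an array of materials.
; BeginPlay applies the material at the current index, and each OnReceiveSignal event advances the index with modulo wraparound and reapplies it through ChangeMaterial.
; Each signal also switches the cube's physics simulation and collision off and immediately back on.
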(event `self.ReceiveBeginPlay`
  ;[1 1 1] Start Param
  (`self.changeMaterial`))

(event `/Game/Blueprints/bpi_signalReeiver.OnReceiveSignal`
  (params (emiter :type "Actor Object Reference") (emitterID :type Byte))
  ;[1 1 1] Change the color
  (bind _result (`/Engine/EditorBlueprintResources/StandardMacros.IncrementInt` (`self.currentMaterialIndex`))
    (:`  `
      (set `self.currentMaterialIndex` (mod _result (`KismetArrayLibrary.Array_Length` (`self.materials`))))
      (`self.changeMaterial`)
      (`PrimitiveComponent.SetSimulatePhysics` (`self.cube`) false)
      (`PrimitiveComponent.SetCollisionEnabled` (`self.cube`) "NoCollision")
      (`PrimitiveComponent.SetCollisionEnabled` (`self.cube`) "QueryAndPhysics")
      (`PrimitiveComponent.SetSimulatePhysics` (`self.cube`) true))))

(fn `changeMaterial`
  (`PrimitiveComponent.SetMaterial` (`self.cube`) 0 (`|GetArrayItem` (`self.materials`) (`self.currentMaterialIndex`))))

(fn `UserConstructionScript`)
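; Controlled platform Blueprint that steps 100 units along a horizontal axis chosen by the ID of the signal emitter it hears.
; On a signal while not already moving, it maps the ID to left, right, forward or backward, stores start and end positions, and sets CanMove.
; Tick only calls the parent, so the movement itself is not in this graph.
; A separate function teleports Plateforme back to BeginPos without sweeping.
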(event `self.ReceiveTick`
  (params (DeltaSeconds :type "Float (single-precision)"))
  (`parent.ReceiveTick` DeltaSeconds))

(event `/Game/Blueprints/bpi_signalReeiver.OnReceiveSignal`
  (params (emiter :type "Actor Object Reference") (emitterID :type Byte))
  (if (not (`self.canMove`))
    (`self.getDirectionById` emitterID)
    (set `self.startPosition` (`self.K2_GetActorLocation`))
    (set `self.endPosition` (+ (* (`self.direction`) 100.0) (`self.K2_GetActorLocation`)))
    (set `self.canMove` true)))

(fn `getDirectionById`
  (params (id :type Byte))
  (if (== id (`self.leftID`))
    (set `self.direction` (0.0 -1.0 0.0))
    (elif (== id (`self.rightID`))
      (set `self.direction` (0.0 1.0 0.0))
      (elif (== id (`self.forwardID`))
        (set `self.direction` (1.0 0.0 0.0))
        (elif (== id (`self.backwardID`))
          (set `self.direction` (-1.0 0.0 0.0)))))))

(fn `GotoInitialePosition `
  (`self.K2_SetActorLocation` (`self.Plateforme`) (`self.BeginPos`) false false))

(fn `UserConstructionScript`
  (`parent.UserConstructionScript`))
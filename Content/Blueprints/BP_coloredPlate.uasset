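; BP_coloredPlate is a color-matched pressure plate that switches a linked object on and off.
; When a component entering its Box trigger shares the Cube's first material, it sends OnStateChangedMessage to ObjectToActivate with IsActivated true and itself as Emitter.
; Any end overlap sends the same message with IsActivated false, without checking the material.
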(event `self.Box.OnComponentBeginOverlap`
  (params (OverlappedComponent :type "PrimitiveComponent Object Reference") (OtherActor :type "Actor Object Reference") (OtherComp :type "PrimitiveComponent Object Reference") (OtherBodyIndex :type Integer) (bFromSweep :type Boolean) (SweepResult :type "HitResult Structure (by ref)"))
  (if (== (`PrimitiveComponent.GetMaterial` OtherComp 0) (`PrimitiveComponent.GetMaterial` (`self.Cube`) 0))
    (message `/Game/Blueprints/BPI_Activable.OnStateChanged` (`self.ObjectToActivate`) true self)))

(event `self.Box.OnComponentEndOverlap`
  (params (OverlappedComponent :type "PrimitiveComponent Object Reference") (OtherActor :type "Actor Object Reference") (OtherComp :type "PrimitiveComponent Object Reference") (OtherBodyIndex :type Integer))
  (message `/Game/Blueprints/BPI_Activable.OnStateChanged` (`self.ObjectToActivate`) false self))

(fn `UserConstructionScript`)
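; Door that rises by an offset to open once enough distinct emitters, such as switches, are active, and returns to its start position to close.
; OnStateChanged tracks active emitters, calling Activate when their count reaches LockedCount and Deactivate on any off signal.
; Both set movement targets and scale travel time by remaining distance, keeping speed consistent when reversed mid-move; the interpolation itself is not in this graph.
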(event `/Game/Blueprints/BPI_Activable.OnStateChanged`
  (params (IsActivated :type Boolean) (emitter :type "Actor Object Reference"))
  ;[1 1 1] Activate/Desactivate Doors
  (if IsActivated
    (if (not (`KismetArrayLibrary.Array_Contains` (`self.unlockedActor`) emitter))
      (`KismetArrayLibrary.Array_Add` (`self.unlockedActor`) emitter)
      (`/Engine/EditorBlueprintResources/StandardMacros.IncrementInt` (`self.unlocked`)
        (:`  `
          (if (== (`self.unlocked`) (`self.lockedCount`))
            (`self.Activate`)))))
    (else
      (if (`KismetArrayLibrary.Array_Contains` (`self.unlockedActor`) emitter)
        (`KismetArrayLibrary.Array_RemoveItem` (`self.unlockedActor`) emitter)
        (`/Engine/EditorBlueprintResources/StandardMacros.DecrementInt` (`self.unlocked`)
          (:`  `
            _)))
      (`self.Deactivate`))))

(event `self.ReceiveBeginPlay`
  (bind (_returnvalue_x _returnvalue_y _returnvalue_z) (`KismetMathLibrary.BreakVector` (`self.K2_GetActorLocation`)))
  ;[1 1 1] Start position
  (set `self.closePos` (`self.K2_GetActorLocation`))
  (set `self.openPos` (`KismetMathLibrary.MakeVector` _returnvalue_x _returnvalue_y (+ _returnvalue_z (`self.openOffset`))))
  (set `self.baseTime` (`self.timeToGo`))
  (set `self.canMove` false))

(fn `Activate`
  (set `self.startPosition` (`self.K2_GetActorLocation`))
  (set `self.endPosition` (`self.openPos`))
  (set `self.canMove` true)
  (set `self.timeAtStart` 0.0)
  (set `self.timeToGo` (* (/ (`KismetMathLibrary.Vector_Distance` (`self.startPosition`) (`self.openPos`)) (`KismetMathLibrary.Vector_Distance` (`self.openPos`) (`self.closePos`))) (`self.baseTime`))))

(fn `Deactivate`
  (set `self.startPosition` (`self.K2_GetActorLocation`))
  (set `self.endPosition` (`self.closePos`))
  (set `self.canMove` true)
  (set `self.timeAtStart` 0.0)
  (set `self.timeToGo` (* (/ (`KismetMathLibrary.Vector_Distance` (`self.startPosition`) (`self.closePos`)) (`KismetMathLibrary.Vector_Distance` (`self.openPos`) (`self.closePos`))) (`self.baseTime`))))

(fn `UserConstructionScript`
  (`parent.UserConstructionScript`))